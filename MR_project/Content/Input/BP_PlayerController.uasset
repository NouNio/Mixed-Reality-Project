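; Player controller that maps left and right trigger input to either hand interaction or movement, depending on a MovementEnabled toggle.
; With movement off, each trigger triggers its hand on press and releases it on completion.
; With movement on, pressing releases that hand and sets NdcBasic's speed backward (left) or forward (right), zeroed on completion.
; The toggle action flips the mode and copies it to both hands.
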(event Input|EnhancedActionEvents|EnhancedInputActionIA_LeftTrigger
  (params (ActionValue :type Boolean) (ElapsedSeconds :type Float%20%28double-precision%29) (TriggeredSeconds :type Float%20%28double-precision%29) (InputAction :type Input%20Action%20Object%20Reference :default "/Game/Input/IA_LeftTrigger.IA_LeftTrigger"))
  (bind _lefthand (Variables|Default|GetLeftHand))
  (bind _ndcbasic (Variables|Default|GetNdcBasic))
  (bind _movementenabled (Variables|Default|GetmovementEnabled))
  (:Started
    (if _movementenabled
      (Utilities|FlowControl|Sequence
        (:then_0
          (Default|Release _lefthand :!label _label))
        (:then_1
          (Variables|/Game/ExampleConfigs/NDC_Basic.NDC_Basic_C|Setspeed _ndcbasic (* (Variables|Default|Getspeed) -1.0))))
      (else
        (Default|Trigger _lefthand))))
  (:Completed
    (if _movementenabled
      (Variables|/Game/ExampleConfigs/NDC_Basic.NDC_Basic_C|Setspeed _ndcbasic 0.0)
      (else
        (goto _label)))))

(event Input|EnhancedActionEvents|EnhancedInputActionIA_RightTrigger
  (params (ActionValue :type Boolean) (ElapsedSeconds :type Float%20%28double-precision%29) (TriggeredSeconds :type Float%20%28double-precision%29) (InputAction :type Input%20Action%20Object%20Reference :default "/Game/Input/IA_RightTrigger.IA_RightTrigger"))
  (bind _righthand (Variables|Default|GetRightHand))
  (bind _ndcbasic (Variables|Default|GetNdcBasic))
  (bind _movementenabled (Variables|Default|GetmovementEnabled))
  (:Started
    (if _movementenabled
      (Utilities|FlowControl|Sequence
        (:then_0
          (Default|Release _righthand :!label _label))
        (:then_1
          (Variables|/Game/ExampleConfigs/NDC_Basic.NDC_Basic_C|Setspeed _ndcbasic (Variables|Default|Getspeed))))
      (else
        (Default|Trigger _righthand))))
  (:Completed
    (if _movementenabled
      (Variables|/Game/ExampleConfigs/NDC_Basic.NDC_Basic_C|Setspeed _ndcbasic 0.0)
      (else
        (goto _label)))))

(event Input|EnhancedActionEvents|EnhancedInputActionIA_MovementToggle
  (params (ActionValue :type Boolean) (ElapsedSeconds :type Float%20%28double-precision%29) (TriggeredSeconds :type Float%20%28double-precision%29) (InputAction :type Input%20Action%20Object%20Reference :default "/Game/Input/IA_MovementToggle.IA_MovementToggle"))
  (:Started
    (bind _output_get (Variables|Default|SetmovementEnabled (not (Variables|Default|GetmovementEnabled))))
    (bind _output_get_2 (Variables|/Game/BP_BaseHandTracked.BP_BaseHandTracked_C|SetmovementEnabled (Variables|Default|GetLeftHand) _output_get))
    (Variables|/Game/BP_BaseHandTracked.BP_BaseHandTracked_C|SetmovementEnabled (Variables|Default|GetRightHand) _output_get_2)))

(event EventBeginPlay)

(event EventTick
  (params (DeltaSeconds :type Float%20%28single-precision%29)))

(fn ConstructionScript)