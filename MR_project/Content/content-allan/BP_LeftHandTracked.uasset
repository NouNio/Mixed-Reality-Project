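; Left-hand actor, apparently for tracked-hand input, that picks a "material" actor by pointing and spawns a copy of it at the hand.
; While nothing is held, Tick line-traces forward on Visibility and stores the hit actor as MaterialHighlight, with a debug line drawn.
; Trigger spawns that actor's class at the hand's transform as MaterialInHand, without attaching it; Release destroys it.
; Unwired copies of both functions remain in the EventGraph.
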(event EventBeginPlay)

(event Collision|EventActorBeginOverlap
  (params (OtherActor :type Actor%20Object%20Reference)))

(event EventTick
  (params (DeltaSeconds :type Float%20%28single-precision%29))
  (bind _returnvalue (Transformation|GetActorLocation))
  (if (not (Utilities|IsValid (Variables|Default|GetMaterialInHand)))
    (bind (_outhit _returnvalue_2) (Collision|LineTraceByChannel _returnvalue (+ _returnvalue (* (Transformation|GetActorForwardVector) (Variables|Default|GetRay%20Length))) "TraceTypeQuery1" false 0 "ForOneFrame"))
    (if _returnvalue_2
      (if (!= (Variables|Default|GetMaterialHighlight) (.HitActor (Collision|BreakHitResult _outhit)))
        (Variables|Default|SetMaterialHighlight (.HitActor (Collision|BreakHitResult _outhit))))
      (else
        (Variables|Default|SetMaterialHighlight 0)))))

(fn ConstructionScript)

(fn Trigger
  (bind _materialhighlight (Variables|Default|GetMaterialHighlight))
  (if (Utilities|IsValid _materialhighlight)
    (bind _returnvalue (Game|SpawnActorfromClass (Utilities|GetClass _materialhighlight) (Transformation|GetActorTransform) "Undefined" "OverrideRootScale" 0 0))
    (bind _output_get (Variables|Default|SetMaterialInHand _returnvalue))
    (Development|PrintString (Utilities|GetDisplayName _output_get))))

(fn Release
  (Actor|DestroyActor (Variables|Default|GetMaterialInHand))
  (bind _output_get (Variables|Default|SetMaterialInHand 0))
  (Development|PrintString (Utilities|GetDisplayName _output_get)))