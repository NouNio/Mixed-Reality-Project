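; Base tracked-hand actor that points at material actors, highlights them and holds a copy of the selected one.
; While empty-handed, Tick traces forward and moves a counter-based overlay highlight between baseclassmaterial hits.
; Trigger spawns a copy of the highlighted class, scaled so its largest bound matches TargetSize.
; Tick keeps that copy at the hand, offset along world X by CombinationPlane, until Release destroys it.
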(event EventBeginPlay)

(event Collision|EventActorBeginOverlap
  (params (OtherActor :type Actor%20Object%20Reference)))

(event EventTick
  (params (DeltaSeconds :type Float%20%28single-precision%29))
  (bind _returnvalue (Transformation|GetActorLocation))
  (bind _materialinhand (Variables|Default|GetMaterialInHand))
  (if (Utilities|IsValid _materialinhand)
    (Transformation|SetActorLocationAndRotation _materialinhand (+ (Transformation|GetActorLocation) (Math|Vector|MakeVector (Variables|Default|GetCombinationPlane) 0.0 0.0)) (Transformation|GetActorRotation))
    (else
      (bind (_outhit _returnvalue_2) (Collision|LineTraceByChannel _returnvalue (+ _returnvalue (* (Transformation|GetActorForwardVector) (Variables|Default|GetRay%20Length))) "TraceTypeQuery1" false 0 (select (Variables|Default|GetmovementEnabled) "None" "ForOneFrame"))) ; IF ray hit,\n\n- check if hit is of baseclassmaterial. If yes, proceed, if not un set material.\n\n- check if stored material highlight is same. If same, do nothing, if different remove material overlay, store into material highlight and highlight new with overlay
      (if _returnvalue_2
        (if (!= (Variables|Default|GetMaterialHighlight) (.HitActor (Collision|BreakHitResult _outhit)))
          (bind _asbaseclassmaterial (Utilities|Casting|CastTobaseclassmaterial (.HitActor (Collision|BreakHitResult _outhit)))
            (:then
              (Utilities|FlowControl|Sequence
                (:then_0
                  (if (Utilities|IsValid (Variables|Default|GetMaterialHighlight)) :!label _label
                    (Variables|/Game/baseclassmaterial.baseclassmaterial_C|Sethighlight%20counter (Variables|Default|GetMaterialHighlight) (- (Variables|/Game/baseclassmaterial.baseclassmaterial_C|Gethighlight%20counter (Variables|Default|GetMaterialHighlight)) 1))
                    (Default|SetOverlay (Variables|Default|GetMaterialHighlight))
                    (Variables|Default|SetMaterialHighlight 0)))
                (:then_1
                  (Variables|/Game/baseclassmaterial.baseclassmaterial_C|Sethighlight%20counter _asbaseclassmaterial (+ (Variables|/Game/baseclassmaterial.baseclassmaterial_C|Gethighlight%20counter _asbaseclassmaterial) 1))
                  (bind _output_get (Variables|Default|SetMaterialHighlight _asbaseclassmaterial))
                  (Default|SetOverlay _output_get))))
            (:CastFailed
              (goto _label))))))))

(fn ConstructionScript)

(fn Trigger
  (bind _materialhighlight (Variables|Default|GetMaterialHighlight))
  (bind _boxextent (Collision|GetActorBounds _materialhighlight false false))
  (bind _returnvalue (* _boxextent "2.000000,2.000000,2.000000"))
  (bind (_x _y _z) (Math|Vector|BreakVector _returnvalue))
  (if (Utilities|IsValid _materialhighlight)
    (bind _returnvalue_2 (Game|SpawnActorfromClass (Utilities|GetClass _materialhighlight) (Math|Transform|MakeTransform (Transformation|GetActorLocation) "0, 0, 0" (* (Transformation|GetActorScale3D _materialhighlight) (/ (Variables|Default|GetTargetSize) (Math|Float|Max(Float) _x _y _z)))) "Undefined" "OverrideRootScale" 0 0))
    (bind _output_get (Variables|Default|SetMaterialInHand _returnvalue_2))))

(fn Release
  (if (Utilities|IsValid (Variables|Default|GetMaterialInHand))
    (Actor|DestroyActor (Variables|Default|GetMaterialInHand)))
  (Variables|Default|SetMaterialInHand 0))