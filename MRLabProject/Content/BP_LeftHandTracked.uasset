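; BP_LeftHandTracked is a Blueprint for the left hand, apparently a tracked one, that registers itself with the player controller.
; On BeginPlay it runs the parent logic, casts player controller 0 to BP_PlayerController and stores itself in that controller's LeftHand variable.
; It adds no other behavior, since its overlap and tick events are disabled and its construction script only calls the parent.
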(event EventBeginPlay
  (|CallParentFunction)
  (bind _asbp_player_controller (Utilities|Casting|CastToBP_PlayerController (Game|GetPlayerController 0)))
  (Variables|/Game/Input/BP_PlayerController.BP_PlayerController_C|SetLeftHand _asbp_player_controller self))

(event Collision|EventActorBeginOverlap
  (params (OtherActor :type Actor%20Object%20Reference))
  (|CallParentFunction OtherActor) ; This node is disabled and will not be called.\nDrag off pins to build functionality.
)

(event EventTick
  (params (DeltaSeconds :type Float%20%28single-precision%29))
  (|CallParentFunction DeltaSeconds) ; This node is disabled and will not be called.\nDrag off pins to build functionality.
)

(fn ConstructionScript
  (|CallParentFunction))